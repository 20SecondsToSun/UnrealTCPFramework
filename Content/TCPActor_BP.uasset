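; TCP server test actor that reports socket activity on screen and shows the server widget.
; On BeginPlay it binds handlers to its TCPServer's listen start, listen stop, socket error, client connected and string received delegates, then adds TCPServer_Windget_BP to the viewport.
; Each handler only prints a message, color-coded for status events and errors, with received strings printed as they arrive.
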(event `self.ReceiveBeginPlay`
  (bind _tcpserver (`self.TCPServer`))
  ;[1 1 1] Main Events
  (add `TCPServerComponent.OnListenSocketStart` _tcpserver (delegate `ServerStartListen`))
  (add `TCPServerComponent.OnListenSocketStop` _tcpserver (delegate `ServerStopListen`))
  (add `TCPServerComponent.OnListenSocketError` (`self.TCPServer`) (delegate `SocketError`))
  (add `TCPServerComponent.OnClientConnected` (`self.TCPServer`) (delegate `Client Connected`))
  (add `TCPServerComponent.OnReceivedString` (`self.TCPServer`) (delegate `onRecvString`))
  ;[1 1 1] UI
  (bind _returnvalue (`|CreateWidget` "/Game/TCPServer_Windget_BP.TCPServer_Windget_BP_C"))
  (`UserWidget.AddToViewport` _returnvalue 0))

(event `ServerStartListen`
  ;[1 1 1] Main Events
  (`KismetSystemLibrary.PrintString` "Server Start Listening" true true (struct :`R` 0.312642 :`G` 1.0 :`A` 1.0)))

(event `ServerStopListen`
  ;[1 1 1] Main Events
  (`KismetSystemLibrary.PrintString` "Server Stop Listening" true true (struct :`R` 1.0 :`G` 0.87614 :`A` 1.0)))

(event `SocketError`
  (params (Error :type "ESocketError Enum" :default "SocketCreationError"))
  ;[1 1 1] Main Events
  (`KismetSystemLibrary.PrintString` (`|GetEnumeratorNameAsString` Error) true true (struct :`R` 1.0 :`B` 0.12942 :`A` 1.0)))

(event `Client Connected`
  (params (Client :type String))
  (`KismetSystemLibrary.PrintString` (`KismetStringLibrary.Concat_StrStr` "Client connected: " Client) true true (struct :`G` 1.0 :`B` 0.126143 :`A` 1.0)))

(event `onRecvString`
  (params (Message :type String))
  (`KismetSystemLibrary.PrintString` Message))

(fn `UserConstructionScript`)